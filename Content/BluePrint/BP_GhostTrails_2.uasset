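; Ghost trail afterimage actor that snapshots the player's pose with a translucent-style material.
; On BeginPlay it casts player pawn 0 to BP_GhostTrailsMesh, stopping if that fails, then gives each material slot of the Fantasminha mesh a dynamic MI_GhostTrails instance and copies the player mesh's pose.
; An Opacity timeline meant to fade those materials and destroy the actor is unconnected, so it never runs.
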(event `self.ReceiveBeginPlay`
  (bind _asbp_ghost_trails_mesh (cast `/Game/BluePrint/BP_GhostTrailsMesh` (`GameplayStatics.GetPlayerPawn` 0)))
  (set `self. PlayerCharacterRef` _asbp_ghost_trails_mesh)
  (`self.GhostTrails`))

(event `GhostTrails`
  (for _ (`MeshComponent.GetMaterials` (`self.Fantasminha`))
    (bind _returnvalue (`KismetMaterialLibrary.CreateDynamicMaterialInstance` "/Game/BluePrint/MI_GhostTrails.MI_GhostTrails"))
    (bind _returnvalue_2 (`KismetArrayLibrary.Array_Add` (`self.DynamicMats`) _returnvalue))
    (`PrimitiveComponent.SetMaterial` (`self.Fantasminha`) _returnvalue_2 _returnvalue)
    (`PoseableMeshComponent.CopyPoseFromSkeletalComponent` (`self.Fantasminha`) (`Character.Mesh` (`self. PlayerCharacterRef`)))))

(fn `UserConstructionScript`)