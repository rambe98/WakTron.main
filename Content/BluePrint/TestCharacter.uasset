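; TestCharacter is a player character Blueprint with movement, mouse look, flight and a ghost-trail spawn.
; Axis inputs drive forward, right and vertical movement relative to control yaw, plus controller yaw and pitch.
; A FlyingKey event feeds a FlipFlop whose only wired branch sets Flying mode, with no switch back.
; Pressing F spawns BP_GhostTrails at the mesh's world transform.
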(event `Key|F`
  (params (Key :type "Key Structure"))
  (:`Pressed`
    (`|SpawnActorFromClass` "/Game/BluePrint/BP_GhostTrails.BP_GhostTrails_C" (`SceneComponent.K2_GetComponentToWorld` (`self.Mesh`)) "Undefined" "OverrideRootScale" null null)))

(event `InputAxis|MoveForward`
  (params (AxisValue :type "Float (single-precision)"))
  ;[1 1 1] 캐릭터 이동
  (`self.AddMovementInput` (`KismetMathLibrary.GetForwardVector` (`KismetMathLibrary.MakeRotator` 0.0 0.0 (.yaw (`self.GetControlRotation`)))) AxisValue))

(event `InputAxis|FlyingKey`
  (params (AxisValue :type "Float (single-precision)"))
  ;[1 1 1] 캐릭터 이동
  (`self.AddMovementInput` (`KismetMathLibrary.GetUpVector` (`KismetMathLibrary.MakeRotator` 0.0 0.0 (.yaw (`self.GetControlRotation`)))) AxisValue))

(event `InputAxis|MoveRight`
  (params (AxisValue :type "Float (single-precision)"))
  ;[1 1 1] 캐릭터 이동
  (`self.AddMovementInput` (`KismetMathLibrary.GetRightVector` (`KismetMathLibrary.MakeRotator` 0.0 0.0 (.yaw (`self.GetControlRotation`)))) AxisValue))

(event `InputAxis|FlyingKey`
  (params (AxisValue :type "Float (single-precision)"))
  ;[1 1 1] 캐릭터 비행
  (`/Engine/EditorBlueprintResources/StandardMacros.FlipFlop`
    (:`A`
      (`CharacterMovementComponent.SetMovementMode` (`self.CharacterMovement`) "MOVE_Flying" 0))))

(event `InputAxis|LookRight`
  (params (AxisValue :type "Float (single-precision)"))
  ;[1 1 1] 마우스 회전
  (`self.AddControllerYawInput` AxisValue))

(event `InputAxis|LookUp`
  (params (AxisValue :type "Float (single-precision)"))
  ;[1 1 1] 마우스 회전
  (`self.AddControllerPitchInput` AxisValue))

(fn `UserConstructionScript`)